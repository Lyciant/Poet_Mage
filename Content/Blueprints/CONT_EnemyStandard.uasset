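; AI controller for standard enemies that runs EnemyStandard_BT and feeds it blackboard keys from perception.
; On possess it sets IsHostile from the pawn's BattleState.
; Sensing a Player-tagged actor cancels the lost-sight timer; losing it starts that timer, which clears SensedActor on expiry.
; The HasLineOfSight and TargetActor setters ignore their inputs, always writing boolean false and true respectively, and UpdateBattleStateKey is empty.
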(event `self.ReceivePossess`
  (params (PossessedPawn :type "Pawn Object Reference"))
  (`self.RunBehaviorTree` "/Game/Blueprints/EnemyStandard_BT.EnemyStandard_BT") ; Select which BHT to use after being used by an actor.
  (`self.UpdateIsHostileKey` (`|EnumEquality` (`/Game/Blueprints/BP_Enemy.battleState` (cast `/Game/Blueprints/BP_EnemyStandard` PossessedPawn :!pure true)) "NewEnumerator0")) ; Set the default value for isHostile to hostile if the enemy is indeed set to hostile on its BP.
)

(event `self.AIPerception.OnTargetPerceptionUpdated`
  (params (Actor :type "Actor Object Reference") (Stimulus :type "AIStimulus Structure"))
  (set `self.sensedActor` Actor)
  (if (`self.ActorHasTag` Actor "Player")
    (if (`.bSuccessfullySensed` (break `AIStimulus` Stimulus))
      (`KismetSystemLibrary.PrintString` "Hello player:")
      (`KismetSystemLibrary.PrintString` (`KismetSystemLibrary.GetObjectName` (`self.sensedActor`)))
      (`KismetSystemLibrary.K2_ClearAndInvalidateTimerHandle` (`self.lostSightHandle`))
      (`self.UpdateHasLineOfSightKey` true)
      (`self.UpdateTargetActorKey` (`self.sensedActor`))
      (else
        (`KismetSystemLibrary.PrintString` "Goodbye")
        ;[1 1 1] If self cannot find player, give up the chase.
        (bind _returnvalue (`KismetSystemLibrary.K2_SetTimerDelegate` (delegate `LostSightOfTarget`) (`self.lostSightTimer`))) ; After Time seconds, fire linked Event. Else, keep running this flow.
        (set `self.lostSightHandle` _returnvalue)
        (`self.UpdateHasLineOfSightKey` false) ; This function tells the code and the BB that we lost line of sight.
      ))
    (else
      (`KismetSystemLibrary.PrintString` "What was sensed was not tagged player"))))

(event `LostSightOfTarget`
  ;[1 1 1] If self cannot find player, give up the chase.
  (`self.UpdateTargetActorKey` null)
  (set `self.sensedActor` null) ; nullify sensed actor variable
)

(fn `UpdateBattleStateKey`
  (params (battleState :type "/Game/Blueprints/Enemy_BattleState Enum" :default "NewEnumerator0")))

(fn `UpdateHasLineOfSightKey`
  (params (hasLineOfSight :type Boolean))
  (`BlackboardComponent.SetValueAsBool` (`AIBlueprintHelperLibrary.GetBlackboard` null) (`self.hasLineOfSight`) false))

(fn `UpdateIsHostileKey`
  (params (isHostile :type Boolean))
  (`BlackboardComponent.SetValueAsBool` (`AIBlueprintHelperLibrary.GetBlackboard` null) (`self.isHostile`) isHostile))

(fn `UpdateTargetActorKey`
  (params (targetActor :type "Actor Object Reference"))
  (`BlackboardComponent.SetValueAsBool` (`AIBlueprintHelperLibrary.GetBlackboard` null) (`self.targetActor`) true))

(fn `UserConstructionScript`)