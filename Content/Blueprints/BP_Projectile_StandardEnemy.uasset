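; BP_Projectile_StandardEnemy is the standard enemy's projectile, which damages the player on contact.
; When its Collision component begins an overlap, it checks for the BPI_Damagable interface and the Player tag, then sends the other actor a DealDamage interface message with its Damage value.
; The graph has no other active gameplay logic, so it does not destroy the projectile on hit.
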(event `self.Collision.OnComponentBeginOverlap`
  (params (OverlappedComponent :type "PrimitiveComponent Object Reference") (OtherActor :type "Actor Object Reference") (OtherComp :type "PrimitiveComponent Object Reference") (OtherBodyIndex :type Integer) (bFromSweep :type Boolean) (SweepResult :type "HitResult Structure (by ref)"))
  (if (`KismetSystemLibrary.DoesImplementInterface` null "/Game/Blueprints/BPI/BPI_Damagable.BPI_Damagable_C")
    ;[1 1 1] Check if you may damage the other actor
    (if (`self.ActorHasTag` (`self.Other Actor`) "Player")
      (message `/Game/Blueprints/BPI/BPI_Damagable.DealDamage` (`self.Other Actor`) (`self.damage`)))))

(fn `UserConstructionScript`
  (`parent.UserConstructionScript`))