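; BP_Enemy is an enemy Blueprint that shows a floating name label and holds a health value.
; The construction script and BeginPlay both set the label from DisplayName, and BeginPlay also resets Health to MaxHealth.
; Each Tick rotates the label to face the player character's camera component.
; No damage or death logic is present, and HealthWidget is unused.
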(event `self.ReceiveBeginPlay`
  (`TextRenderComponent.K2_SetText` (`self.Name`) (`KismetTextLibrary.Conv_StringToText` (`self.displayName`)))
  (`self.ResetHealth`))

(event `self.ReceiveTick`
  (params (DeltaSeconds :type "Float (single-precision)"))
  (`self.AlignNameWithCamera`))

(fn `AlignNameWithCamera`
  (`SceneComponent.K2_SetWorldRotation` (`self.Name`) (`KismetMathLibrary.FindLookAtRotation` (`SceneComponent.K2_GetComponentLocation` (`self.Name`)) (`SceneComponent.K2_GetComponentLocation` (`self.GetComponentByClass` (`GameplayStatics.GetPlayerCharacter` 0) "/Script/Engine.CameraComponent"))) false false))

(fn `ResetHealth`
  (set `self._health` (`self.maxHealth`)))

(fn `UserConstructionScript`
  ;[1 1 1] Set name
  (`TextRenderComponent.K2_SetText` (`self.Name`) (`KismetTextLibrary.Conv_StringToText` (`self.displayName`))))